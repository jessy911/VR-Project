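; Wand projectile that knocks a flag crystal out of the inventory of the VR character it hits.
; On sphere hit, it takes the first actor attached to that character's inventory child actor and, if it is a flag crystal, calls its SpawnFlag.
; ServerDeleteChrystal then destroys the crystal, disables collision, plays smoke and eject sound at the impact, and destroys the projectile.
; Any other hit is ignored.
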(event `self.Sphere.OnComponentHit`
  (params (HitComponent :type "PrimitiveComponent Object Reference") (OtherActor :type "Actor Object Reference") (OtherComp :type "PrimitiveComponent Object Reference") (NormalImpulse :type "Vector Structure") (Hit :type "HitResult Structure (by ref)"))
  (bind _asbp_vrcharacter (cast `/Game/NewCharacter/BP_VRCharacter` OtherActor))
  (bind _output (`|GetArrayItem` (`self.GetAttachedActors` (`ChildActorComponent.ChildActor` (`/Game/NewCharacter/BP_VRCharacter.Inventory` _asbp_vrcharacter)) true false)))
  (bind _asbp_flag_crystal (cast `/Game/Inventory/Blueprints/BP_FlagCrystal` _output))
  (`/Game/Inventory/Blueprints/BP_FlagCrystal.SpawnFlag` _asbp_flag_crystal)
  (`self.ServerDeleteChrystal` Hit _output))

(event `ServerDeleteChrystal`
  (params (HitNode :type "HitResult Structure") (Chrystal :type "Actor Object Reference"))
  (bind (_bblockinghit _binitialoverlap _time _distance _location _impactpoint _normal) (`GameplayStatics.BreakHitResult` HitNode))
  (`self.K2_DestroyActor` Chrystal)
  (`PrimitiveComponent.SetCollisionEnabled` (`self.Sphere`) "NoCollision")
  (`GameplayStatics.SpawnEmitterAtLocation` "/Game/HandPaintedEnvironment/Assets/Particles/Smoke.Smoke" _location (`KismetMathLibrary.MakeRotFromX` _normal))
  (`GameplayStatics.PlaySoundAtLocation` "/Engine/EditorSounds/GamePreview/EjectFromPlayer.EjectFromPlayer" _location (struct) 1.0 1.0 0.0 null null null null)
  (`self.K2_DestroyActor`))

(fn `UserConstructionScript`)