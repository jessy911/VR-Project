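; BP_CollisionTarget is a goal zone in the summer scene that declares a win when a VR player brings in a flag crystal.
; On sphere overlap it searches the actors attached to that BP_VRCharacter's inventory child actor for a BP_FlagCrystal.
; For each crystal found, it calls ShowWinnerWidget on every BP_VRCharacter in the world.
; The server and multicast widget-spawn events are empty, and their spawn logic is disconnected.
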(event `self.Sphere.OnComponentBeginOverlap`
  (params (OverlappedComponent :type "PrimitiveComponent Object Reference") (OtherActor :type "Actor Object Reference") (OtherComp :type "PrimitiveComponent Object Reference") (OtherBodyIndex :type Integer) (bFromSweep :type Boolean) (SweepResult :type "HitResult Structure (by ref)"))
  (bind _asbp_vrcharacter (cast `/Game/NewCharacter/BP_VRCharacter` OtherActor))
  (set `self.PlayerNumberBP` (`KismetTextLibrary.Conv_ObjectToText` _asbp_vrcharacter))
  (for _array_element (`self.GetAttachedActors` (`ChildActorComponent.ChildActor` (`/Game/NewCharacter/BP_VRCharacter.Inventory` _asbp_vrcharacter)) true false)
    (cast `/Game/Inventory/Blueprints/BP_FlagCrystal` _array_element)
    (bind _outactors (`GameplayStatics.GetAllActorsOfClass` "/Game/NewCharacter/BP_VRCharacter.BP_VRCharacter_C"))
    (for _array_element_2 _outactors
      (`/Game/NewCharacter/BP_VRCharacter.ShowWinnerWidget` _array_element_2))))

(event `ServerSpawnWidget`)

(event `Multicast_SpawnWidget`)

(fn `UserConstructionScript`)