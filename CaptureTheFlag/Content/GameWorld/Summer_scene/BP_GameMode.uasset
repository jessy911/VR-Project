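; Game mode for the Summer scene that assigns spawn points from actors tagged "Player", gathered at BeginPlay.
; Its ChoosePlayerStart override re-gathers them on the first call, sets a ServerIn flag, and begins a random-swap loop that returns within its first iteration.
; Each call increments PlayerID before indexing the array, so later players receive successive entries.
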(event `self.ReceiveBeginPlay`
  (`parent.ReceiveBeginPlay`)
  (bind _outactors (`GameplayStatics.GetAllActorsWithTag` "Player"))
  (set `self.PlayerPosition` _outactors))

(fn `ChoosePlayerStart`
  (params (Player :type "Controller Object Reference"))
  (returns (ReturnValue :type "Actor Object Reference"))
  (bind _playerid (`self.PlayerID`))
  (bind _playerid_2 (`self.PlayerID`))
  (if (`self.ServerIn`)
    (set `self.PlayerID` (+ _playerid 1))
    (return (`|GetArrayItem` (`self.PlayerPosition`) _playerid))
    (else
      (bind _outactors (`GameplayStatics.GetAllActorsWithTag` "Player"))
      (bind _output_get (set `self.PlayerPosition` _outactors))
      (set `self.ServerIn` true)
      (for (_ _array_index) _output_get
        (`KismetArrayLibrary.Array_Swap` _output_get _array_index (`.OutIndex` (`KismetArrayLibrary.Array_Random` (`self.LenPlayer`))))
        (set `self.PlayerID` (+ _playerid_2 1))
        (return (`|GetArrayItem` (`self.PlayerPosition`) _playerid_2))))))

(fn `UserConstructionScript`
  (`parent.UserConstructionScript`))