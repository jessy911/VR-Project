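; Inventory component that lets the player pick up nearby BP_Flag items and view them in a WB_Inventory widget.
; BeginPlay creates and loads the widget, and the left menu input toggles it on the viewport.
; Either grab input runs a debug-drawn sphere trace below the player's location; a flag whose name matches Items overwrites Items, refreshes the widget and is destroyed.
; A BP_Inventory actor spawn is left unconnected.
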(event `self.ReceiveBeginPlay`
  (bind _returnvalue (`|CreateWidget` "/Game/Inventory/Widgets/WB_Inventory.WB_Inventory_C"))
  (bind _output_get (set `self.WB_Inventory` _returnvalue))
  (`/Game/Inventory/Widgets/WB_Inventory.LoadInventory` _output_get self))

(event `EnhancedInput|/Game/VRTemplate/Input/Actions/IA_Menu_Toggle_Left`
  (params (ActionValue :type Boolean) (ElapsedSeconds :type "Float (double-precision)") (TriggeredSeconds :type "Float (double-precision)") (InputAction :type "InputAction Object Reference" :default "/Game/VRTemplate/Input/Actions/IA_Menu_Toggle_Left.IA_Menu_Toggle_Left"))
  (bind _wb_inventory (`self.WB_Inventory`))
  (:`Triggered`
    (if (`Widget.IsVisible` (`self.WB_Inventory`))
      (`Widget.RemoveFromParent` _wb_inventory)
      (else
        (`UserWidget.AddToViewport` _wb_inventory 0)))))

(event `EnhancedInput|/Game/VRTemplate/Input/Actions/IA_Grab_Left_Pressed`
  (params (ActionValue :type "Float (double-precision)") (ElapsedSeconds :type "Float (double-precision)") (TriggeredSeconds :type "Float (double-precision)") (InputAction :type "InputAction Object Reference" :default "/Game/VRTemplate/Input/Actions/IA_Grab_Left_Pressed.IA_Grab_Left_Pressed"))
  (bind _returnvalue (- (`Actor.K2_GetActorLocation` (`GameplayStatics.GetPlayerCharacter` 0)) (0.0 0.0 40.0)))
  (:`Triggered`
    (`KismetSystemLibrary.PrintText` "Left Grab" true true (struct :`G` 0.66 :`B` 1.0 :`A` 1.0) 200.0)
    (bind _outhit (`KismetSystemLibrary.SphereTraceSingle` :`Start` _returnvalue :`End` _returnvalue :`Radius` 120.0 :`TraceChannel` "TraceTypeQuery1" :`DrawDebugType` "ForDuration" :!label _label))
    (bind _asbp_flag (cast `/Game/Inventory/Blueprints/BP_Flag` (`.HitActor` (`GameplayStatics.BreakHitResult` _outhit))))
    (`/Engine/EditorBlueprintResources/StandardMacros.IsValid` _asbp_flag
      (:`Is Valid`
        (if (`KismetTextLibrary.EqualEqual_TextText` (`.Name_2_C0AD66514F04B86060E11D9BEE522B30` (break `/Game/Inventory/Blueprints/S_ItemStructure` (`self.Items`))) (`.Name_2_C0AD66514F04B86060E11D9BEE522B30` (break `/Game/Inventory/Blueprints/S_ItemStructure` (`/Game/Inventory/Blueprints/BP_Flag.Item` _asbp_flag))))
          (bind (_item_name _item_stackable _item_thumnail _item_mesh) (break `/Game/Inventory/Blueprints/S_ItemStructure` (`/Game/Inventory/Blueprints/BP_Flag.Item` _asbp_flag)))
          (set `self.Items` (make `/Game/Inventory/Blueprints/S_ItemStructure` _item_name _item_stackable _item_thumnail _item_mesh))
          (`/Game/Inventory/Widgets/WB_Inventory.LoadInventory` (`self.WB_Inventory`) self)
          (`Actor.K2_DestroyActor` _asbp_flag))))))

(event `EnhancedInput|/Game/VRTemplate/Input/Actions/IA_Grab_Right_Pressed`
  (params (ActionValue :type "Float (double-precision)") (ElapsedSeconds :type "Float (double-precision)") (TriggeredSeconds :type "Float (double-precision)") (InputAction :type "InputAction Object Reference" :default "/Game/VRTemplate/Input/Actions/IA_Grab_Right_Pressed.IA_Grab_Right_Pressed"))
  (:`Triggered`
    (`KismetSystemLibrary.PrintText` "Right Grab" true true (struct :`R` 1.0 :`A` 1.0) 200.0)
    (goto _label)))