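; BP_InventorySlot is a sphere-shaped inventory slot that holds one grabbable object.
; Overlapping actors have their GrabComponent grab and drop events bound, and the sphere enlarges as a highlight.
; Dropping an object into an empty slot disables its physics, snaps it to the overlap sphere and rescales it relative to the slot.
; Grabbing it or ending overlap detaches it and restores its original scale.
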(event `self.ReceiveBeginPlay`
  (set `self.InitialSphereScale` (`SceneComponent.K2_GetComponentScale` (`self.Sphere`))))

(event `self.Sphere1.OnComponentBeginOverlap`
  (params (OverlappedComponent :type "PrimitiveComponent Object Reference") (OtherActor :type "Actor Object Reference") (OtherComp :type "PrimitiveComponent Object Reference") (OtherBodyIndex :type Integer) (bFromSweep :type Boolean) (SweepResult :type "HitResult Structure (by ref)"))
  (for _array_element (`self.K2_GetComponentsByClass` OtherActor "/Game/VRTemplate/Blueprints/GrabComponent.GrabComponent_C")
    (`KismetArrayLibrary.Array_Add` (`self.TrackedGrabComponent`) _array_element)
    (add `/Game/VRTemplate/Blueprints/GrabComponent.OnGrabbed` _array_element (delegate `OnGrabbed_Event`))
    (add `/Game/VRTemplate/Blueprints/GrabComponent.OnDropped` _array_element (delegate `OnDropped_Event`)))
  (`self.IncreaseCellSize`))

(event `OnGrabbed_Event`
  (params (SelfReference :type "/Game/VRTemplate/Blueprints/GrabComponent Object Reference"))
  (`self.TryDropObject` (`ActorComponent.GetOwner` SelfReference)))

(event `OnDropped_Event`
  (params (SelfReference :type "/Game/VRTemplate/Blueprints/GrabComponent Object Reference"))
  (`self.TryCaptureObject` SelfReference)
  (`self.DecreseCellSize`))

(event `self.Sphere1.OnComponentEndOverlap`
  (params (OverlappedComponent :type "PrimitiveComponent Object Reference") (OtherActor :type "Actor Object Reference") (OtherComp :type "PrimitiveComponent Object Reference") (OtherBodyIndex :type Integer))
  (`self.TryDropObject` OtherActor)
  (for _array_element (`self.K2_GetComponentsByClass` OtherActor "/Game/VRTemplate/Blueprints/GrabComponent.GrabComponent_C")
    (`KismetArrayLibrary.Array_RemoveItem` (`self.TrackedGrabComponent`) _array_element)
    (remove `/Game/VRTemplate/Blueprints/GrabComponent.OnGrabbed` _array_element (delegate `OnGrabbed_Event`))
    (remove `/Game/VRTemplate/Blueprints/GrabComponent.OnDropped` _array_element (delegate `OnDropped_Event`)))
  (`self.DecreseCellSize`))

(fn `DecreseCellSize`
  (`SceneComponent.SetWorldScale3D` (`self.Sphere`) (`self.InitialSphereScale`)))

(fn `IncreaseCellSize`
  (`SceneComponent.SetWorldScale3D` (`self.Sphere`) (* (`self.InitialSphereScale`) 1.2)))

(fn `TryCaptureObject`
  (params (`GrabComponent ` :type "/Game/VRTemplate/Blueprints/GrabComponent Object Reference"))
  (`/Engine/EditorBlueprintResources/StandardMacros.IsValid` (`self.HeldActor`)
    (:`Is Not Valid`
      (bind _output_get (set `self.HeldActor` (`ActorComponent.GetOwner` `GrabComponent `)))
      (set `self.InitialActorScale` (`self.GetActorScale3D` _output_get))
      (`/Game/VRTemplate/Blueprints/GrabComponent.SetPrimitiveCompPhysics` `GrabComponent ` false)
      (`self.K2_AttachToComponent` _output_get (`self.Sphere1`) "None" "SnapToTarget" "KeepWorld" "KeepWorld" true)
      (`self.SetActorScale3D` (`self.HeldActor`) (* (`self.InitialSphereScale`) 0.7)))))

(fn `TryDropObject`
  (params (Actor :type "Actor Object Reference"))
  (bind _heldactor (`self.HeldActor`))
  (`/Engine/EditorBlueprintResources/StandardMacros.IsValid` _heldactor
    (:`Is Valid`
      (if (== Actor _heldactor)
        (if (== (`self.GetAttachParentActor` (`self.HeldActor`)) self)
          (`self.K2_DetachFromActor` (`self.HeldActor`) "KeepWorld" "KeepWorld" "KeepWorld"))
        (`self.SetActorScale3D` (`self.HeldActor`) (`self.InitialActorScale`))
        (set `self.HeldActor` null)))))

(fn `UserConstructionScript`)