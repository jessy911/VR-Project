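; Minimap Blueprint that displays a minimap material through a widget component.
; On BeginPlay it casts the component's widget to WBP_Minimap and sets its image brush to M_Minimap.
; RotateMainMenu, which nothing in this Blueprint calls, eases the actor toward the player camera manager's location and yaw, with position lagging well behind the faster rotation.
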(event `self.ReceiveBeginPlay`
  (bind _aswbp_minimap (cast `/Game/MiniMap/WBP_Minimap` (`WidgetComponent.GetUserWidgetObject` (`self.Minimap`))))
  (`Image.SetBrushFromMaterial` (`/Game/MiniMap/WBP_Minimap.Image_0` _aswbp_minimap) "/Game/MiniMap/M_Minimap.M_Minimap"))

(event `self.ReceiveTick`
  (params (DeltaSeconds :type "Float (single-precision)")))

(fn `RotateMainMenu`
  (params (DeltaTime :type "Float (double-precision)"))
  (bind _defaultsceneroot (`self.DefaultSceneRoot`))
  (bind _transformcomponent (`PlayerCameraManager.TransformComponent` (`GameplayStatics.GetPlayerCameraManager` 0)))
  (bind (_returnvalue_roll _returnvalue_pitch _returnvalue_yaw) (`KismetMathLibrary.BreakRotator` (`KismetMathLibrary.RInterpTo` (`SceneComponent.K2_GetComponentRotation` _defaultsceneroot) (`SceneComponent.K2_GetComponentRotation` _transformcomponent) DeltaTime 15.0)))
  (`self.K2_SetActorTransform` (`KismetMathLibrary.MakeTransform` (`KismetMathLibrary.VInterpTo` (`SceneComponent.K2_GetComponentLocation` _defaultsceneroot) (`SceneComponent.K2_GetComponentLocation` _transformcomponent) DeltaTime 0.6) (`KismetMathLibrary.MakeRotator` 0.0 0.0 _returnvalue_yaw))))

(fn `UserConstructionScript`)